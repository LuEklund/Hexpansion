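; BP_EnemyBase is an enemy base actor that travels along a spline with a wobbling mesh.
; Unless stunned, Tick advances distance by ActorSpeed and sets location from the spline plus a world X offset, taking pitch and yaw from the spline.
; A self-restarting Wiggle timeline rolls the mesh.
; Underground hiding and speed switching, map lookup and chunk-to-chunk stepping are present but disconnected.
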(event Custom|Start%20Wiggle
  (bind _returnvalue (Transformation|GetActorTransform))
  (bind _wiggles (Timeline|Wiggle PlayFromStart)
    (:Update
      (Transformation|SetWorldRotation (Variables|Character|GetMesh) (Math|Rotator|MakeRotator (* _wiggles 45.0) (.pitch (.rotation _returnvalue)) (.yaw (.rotation _returnvalue))) false false))
    (:Finished
      (CallFunction|StartWiggle))))

(event EventBeginPlay
  (CallFunction|StartWiggle))

(event EventTick
  (params (DeltaSeconds :type Float%20%28single-precision%29))
  (bind _returnvalue (Transformation|GetActorTransform))
  (if (not (Variables|Default|GetbIsStunned))
    ;[1 1 1] Follow Spline
    (Variables|Default|SetDistanceTraveled (+ (* DeltaSeconds (Variables|Default|GetActorSpeed)) (Variables|Default|GetDistanceTraveled)))
    (Transformation|SetActorTransform (Math|Transform|MakeTransform (+ (Math|Vector|MakeVector (Variables|Default|GetSplineOffset self) 0.0 0.0) (.location (Spline|GetTransformatDistanceAlongSpline (Variables|Default|GetSpline) (Variables|Default|GetDistanceTraveled) "World" true))) (Math|Rotator|MakeRotator (.roll (.rotation _returnvalue)) (.pitch (.rotation (Spline|GetTransformatDistanceAlongSpline (Variables|Default|GetSpline) (Variables|Default|GetDistanceTraveled) "World" true))) (.yaw (.rotation (Spline|GetTransformatDistanceAlongSpline (Variables|Default|GetSpline) (Variables|Default|GetDistanceTraveled) "World" true)))) (.scale _returnvalue)))))

(fn ConstructionScript)

(fn SetSpeed
  (params (Speed :type Float%20%28double-precision%29))
  (Variables|Default|SetActorSpeed Speed))