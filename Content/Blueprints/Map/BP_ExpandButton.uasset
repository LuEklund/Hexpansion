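; BP_ExpandButton is a map button actor that shows a label for its type while the cursor hovers over it.
; On BeginPlay it binds the cursor-over events and hides its InfoWidgetComponent's widget.
; Hovering shows the WBP_ExandInfo widget and sets its text from MyType, covering attack upgrades, boss, special effect and gold; leaving hides it.
; No click or expansion logic is implemented in this Blueprint.
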(event Custom|OnBeginCursorOver_Event
  (params (TouchedActor :type Actor%20Object%20Reference))
  (Widget|SetVisibility (UserInterface|GetWidget (Variables|Default|GetInfoWidgetComponent)) "Visible")
  (bind _aswbp_exand_info (Utilities|Casting|CastToWBP_ExandInfo (UserInterface|GetWidget (Variables|Default|GetInfoWidgetComponent))))
  (switch Utilities|FlowControl|Switch|SwitchonEUpgradeType (Variables|Default|GetMyType)
    (:UTILITY_ATTACK_RANGE
      (Variables|/Script/UMG.TextBlock|SetText (Variables|/Game/Blueprints/UI/Widget/WBP_ExandInfo.WBP_ExandInfo_C|GetTypeText _aswbp_exand_info) "Attack Range"))
    (:UTILITY_ATTACK_SPEED
      (Variables|/Script/UMG.TextBlock|SetText (Variables|/Game/Blueprints/UI/Widget/WBP_ExandInfo.WBP_ExandInfo_C|GetTypeText _aswbp_exand_info) "Attack Speed"))
    (:DAMAGE
      (Variables|/Script/UMG.TextBlock|SetText (Variables|/Game/Blueprints/UI/Widget/WBP_ExandInfo.WBP_ExandInfo_C|GetTypeText _aswbp_exand_info) "Attack Damage"))
    (:BOSS
      (Variables|/Script/UMG.TextBlock|SetText (Variables|/Game/Blueprints/UI/Widget/WBP_ExandInfo.WBP_ExandInfo_C|GetTypeText _aswbp_exand_info) "Boss"))
    (:SPECIAL_EFFECT
      (Variables|/Script/UMG.TextBlock|SetText (Variables|/Game/Blueprints/UI/Widget/WBP_ExandInfo.WBP_ExandInfo_C|GetTypeText _aswbp_exand_info) "Special Effect"))
    (:GOLD
      (Variables|/Script/UMG.TextBlock|SetText (Variables|/Game/Blueprints/UI/Widget/WBP_ExandInfo.WBP_ExandInfo_C|GetTypeText _aswbp_exand_info) "Gold"))))

(event Custom|OnEndCursorOver_Event
  (params (TouchedActor :type Actor%20Object%20Reference))
  (Widget|SetVisibility (UserInterface|GetWidget (Variables|Default|GetInfoWidgetComponent)) "Hidden"))

(event EventBeginPlay
  (EventDispatchers|BindEventtoOnBeginCursorOver (delegate Custom|OnBeginCursorOver_Event))
  (EventDispatchers|BindEventtoOnEndCursorOver (delegate Custom|OnEndCursorOver_Event))
  (Widget|SetVisibility (UserInterface|GetWidget (Variables|Default|GetInfoWidgetComponent)) "Hidden"))

(event Collision|EventActorBeginOverlap
  (params (OtherActor :type Actor%20Object%20Reference)))

(event EventTick
  (params (DeltaSeconds :type Float%20%28single-precision%29)))

(fn ConstructionScript)